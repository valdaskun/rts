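; Construction proxy actor that stands in for an RTS building under construction, showing its display mesh with a ghost material.
; On Tick it advances a clockwork timer scaled by a time unit and compares the work time spent with the construction time set from work hours.
; It registers with MyGameState2 for game speed updates.
; When finished, it broadcasts ConstructionCompleted and destroys itself after a short delay.
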(event `self.ReceiveBeginPlay`
  (bind _output_get (set `self.GameStateReference` (cast `/Game/rts/GameBP/MyGameState2` (`GameplayStatics.GetGameState`) :!pure true)))
  (add `/Game/rts/GameBP/MyGameState2.UpdateGameSpeed` _output_get (`|CreateDelegate` :!event `AjustTime`)))

(event `self.ReceiveTick`
  (params (DeltaSeconds :type "Float (single-precision)"))
  (set `self.Delta` DeltaSeconds)
  (if (not (`self.IsConstructionCompleted`))
    (`self.DoWork`)
    (if (>= (`self.WorkTimeSpent`) (`self.ConstructionTime`))
      (set `self.IsConstructionCompleted` true)
      (`self.ConstructionCompleted` self)
      (`KismetSystemLibrary.Delay` 0.2)
      (`self.K2_DestroyActor`))))

(event `AjustTime`
  (params (TimeUnit :type "Float (double-precision)"))
  (set `self.TimeUnit` TimeUnit))

(fn `DoWork`
  (bind _output_get (set `self.ClockWork` (`/Game/rts/Libraries/FunctionLibrary.SetClockWork` (`self.Delta`) (`self.TimeUnit`) (`self.ClockWork`))))
  (set `self.WorkTimeSpent` (* _output_get 60.0)))

(fn `SetConstructionTime`
  (params (WorkHours :type "Float (double-precision)"))
  (set `self.ConstructionTime` (* WorkHours 60.0))
  (return))

(fn `UserConstructionScript`
  (bind _staticmesh (`self.StaticMesh`))
  (`StaticMeshComponent.SetStaticMesh` _staticmesh (`self.DisplayMesh`))
  (`PrimitiveComponent.SetMaterial` _staticmesh 0 "/Game/rts/Materials/Ghost_Mat_Inst.Ghost_Mat_Inst"))