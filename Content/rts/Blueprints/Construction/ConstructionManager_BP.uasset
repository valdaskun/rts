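; Construction manager for an RTS that turns queued build orders into finished buildings.
; QueueConstruction spawns a ghost-material proxy with the order's display mesh and required working hours, storing order and proxy in parallel arrays.
; It binds to the proxy's ConstructionCompleted event.
; FinnishConstruction finds the order by the proxy's index, removes both entries, spawns the building at the stored transform and destroys the proxy.
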(event `BindConstructionComplete`
  (params (Proxy :type "/Game/rts/Blueprints/Construction/ConstructionProxy_BP Object Reference"))
  (add `/Game/rts/Blueprints/Construction/ConstructionProxy_BP.ConstructionCompleted` Proxy (`|CreateDelegate` :!event `ConstructionCompleted`)))

(event `ConstructionCompleted`
  (params (Proxy :type "/Game/rts/Blueprints/Construction/ConstructionProxy_BP Object Reference"))
  (`self.FinnishConstruction` Proxy))

(fn `FinnishConstruction`
  (params (Proxy :type "/Game/rts/Blueprints/Construction/ConstructionProxy_BP Object Reference"))
  (locals (Index :type Integer :default 0) (Config :type "/Game/rts/Strucs/Construction Structure"))
  (bind _proxies (`self.Proxies`))
  (bind _queue (`self.Queue`))
  (bind _index (`local.Index`))
  (bind (_buildingclass _proxyclass _transform) (break `/Game/rts/Strucs/Construction` (`local.Config`)))
  (bind _output_get (set `local.Index` (`KismetArrayLibrary.Array_Find` _proxies Proxy)))
  (set `local.Config` (`KismetArrayLibrary.Array_Get` _queue _output_get))
  (`KismetArrayLibrary.Array_Remove` _queue _index)
  (`KismetArrayLibrary.Array_Remove` _proxies _index)
  (`|SpawnActorFromClass` _buildingclass _transform "Undefined" "OverrideRootScale")
  (`self.K2_DestroyActor` Proxy))

(fn `QueueConstruction`
  (params (ConstructionStruct :type "/Game/rts/Strucs/Construction Structure"))
  (bind (_buildingclass _proxyclass _transform _displaymesh _workinghoursrequired) (break `/Game/rts/Strucs/Construction` ConstructionStruct))
  (bind _returnvalue (`|SpawnActorFromClass` _proxyclass _transform "AlwaysSpawn" "OverrideRootScale" null _displaymesh))
  (`PrimitiveComponent.SetMaterial` (`/Game/rts/Blueprints/Construction/ConstructionProxy_BP.StaticMesh` _returnvalue) 0 "/Game/rts/Materials/Ghost_Mat_Inst3.Ghost_Mat_Inst3")
  (`self.BindConstructionComplete` _returnvalue)
  (`KismetArrayLibrary.Array_Add` (`self.Proxies`) _returnvalue)
  (`KismetArrayLibrary.Array_Add` (`self.Queue`) ConstructionStruct)
  (`/Game/rts/Blueprints/Construction/ConstructionProxy_BP.SetConstructionTime` _returnvalue _workinghoursrequired))

(fn `UserConstructionScript`)