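; RTS player controller that drives the camera pawn and handles building placement.
; On BeginPlay it spawns a construction manager and ghost building, then creates the main HUD.
; In build mode the ghost follows the cursor and rotates while keys are held; a non-overlapping click queues construction.
; Camera input covers zoom-scaled movement with a Shift boost, screen-edge scrolling, spring-arm zoom, and gated mouse panning that suspends navigation.
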(event `self.ReceiveBeginPlay`
  (bind _returnvalue (`KismetMathLibrary.MakeTransform` (0.0 0.0 0.0)))
  ;[1 1 1] References
  (`|ExecutionSequence`
    (:`then_0`
      (`self.ReferencesCasts`))
    (:`then_1`
      (bind _returnvalue_2 (`|SpawnActorFromClass` "/Game/rts/Blueprints/Construction/ConstructionManager_BP.ConstructionManager_BP_C" _returnvalue "AlwaysSpawn" "OverrideRootScale"))
      (set `self.Construction Manager Ref` _returnvalue_2))
    (:`then_2`
      (bind _returnvalue_3 (`|SpawnActorFromClass` "/Game/rts/Blueprints/Buildings/GhostBuiding_BP.GhostBuiding_BP_C" _returnvalue "AlwaysSpawn" "OverrideRootScale" null self))
      (set `self.Ghost Building Ref` _returnvalue_3))
    (:`then_3`
      (`WidgetBlueprintLibrary.SetInputMode_GameAndUIEx` self null "LockAlways" false)
      (`self.CreateHuds`)
      (`UserWidget.AddToViewport` (`self.MainHudRef`) 0))))

(event `Key|LeftMouseButton`
  (params (Key :type "Key Structure" :default "AnyKey"))
  ;[1 1 1] Place Building
  (:`Pressed`
    (if (and (`self.BuildModeActive`) (not (`/Game/rts/Blueprints/Buildings/GhostBuiding_BP.GetIsOverlapping` (`self.Ghost Building Ref`))))
      (bind _constructionstruct (`/Game/rts/Blueprints/Buildings/GhostBuiding_BP.GetConstructionStruct` (`self.Ghost Building Ref`)))
      (`/Game/rts/Blueprints/Construction/ConstructionManager_BP.QueueConstruction` (`self.Construction Manager Ref`) _constructionstruct)
      (`/Game/rts/Blueprints/Buildings/GhostBuiding_BP.KillGhost` (`self.Ghost Building Ref`)))))

(event `self.ReceiveTick`
  (params (DeltaSeconds :type "Float (single-precision)"))
  ;[1 1 1] Buildings
  (if (`self.BuildModeActive`)
    (if (!= (`self.Ghost Building Ref`) null)
      (`/Game/rts/Blueprints/Buildings/GhostBuiding_BP.SetCursorPosition` (`self.Ghost Building Ref`) (`/Game/rts/Libraries/FunctionLibrary.SetCursorWorldPosition` self (`self.SetSiteDistance`))))))

(event `InputAction|Deselect`
  (params (Key :type "Key Structure" :default "AnyKey"))
  ;[1 1 1] Buildings
  (:`Pressed`
    (if (`self.BuildModeActive`)
      (`/Game/rts/Blueprints/Buildings/GhostBuiding_BP.KillGhost` (`self.Ghost Building Ref`))
      (set `self.BuildModeActive` false))))

(event `InputAction|RotateBuildingRight`
  (params (Key :type "Key Structure" :default "AnyKey"))
  (bind _ghost_building_ref (`self.Ghost Building Ref`))
  (bind (_returnvalue_roll _returnvalue_pitch _returnvalue_yaw) (`KismetMathLibrary.BreakRotator` (`self.K2_GetActorRotation` _ghost_building_ref)))
  ;[1 1 1] Place Building
  (:`Pressed`
    (if (and (`KismetSystemLibrary.IsValid` _ghost_building_ref) (`self.BuildModeActive`)) :!label _label
      (set `self.TurningRight` true)
      (`self.K2_SetActorRotation` _ghost_building_ref (`KismetMathLibrary.MakeRotator` _returnvalue_roll _returnvalue_pitch (- _returnvalue_yaw (`self.BuildingRotationRate`))) false)
      (`KismetSystemLibrary.Delay` 0.1)
      (if (`self.TurningRight`)
        (goto _label))))
  (:`Released`
    (set `self.TurningRight` false)))

(event `InputAxis|MoveForward2`
  (params (AxisValue :type "Float (single-precision)"))
  (bind _camerapawnreference (`self.CameraPawnReference`))
  ;[1 1 1] Camera Movement
  ;;[1 1 1] Move up/down
  (if (not (`self.DisableCamNav`))
    (`self.K2_SetActorTransform` _camerapawnreference (`self.MovementX` (`self.MovementSpeedCalculation`) (`self.FastMoveMultiplier`) AxisValue _camerapawnreference) false false)))

(event `InputAxis|MoveRight`
  (params (AxisValue :type "Float (single-precision)"))
  (bind _camerapawnreference (`self.CameraPawnReference`))
  ;[1 1 1] Camera Movement
  ;;[1 1 1] Move left/right
  (if (not (`self.DisableCamNav`))
    (`self.K2_SetActorTransform` _camerapawnreference (`KismetMathLibrary.MakeTransform` (`KismetMathLibrary.MakeVector` (.x (.location (`self.MovementY` (`self.MovementSpeedCalculation`) (`self.FastMoveMultiplier`) AxisValue _camerapawnreference))) (.y (.location (`self.MovementY` (`self.MovementSpeedCalculation`) (`self.FastMoveMultiplier`) AxisValue _camerapawnreference))) 100.0) (.rotation (`self.MovementY` (`self.MovementSpeedCalculation`) (`self.FastMoveMultiplier`) AxisValue _camerapawnreference)) (.scale (`self.MovementY` (`self.MovementSpeedCalculation`) (`self.FastMoveMultiplier`) AxisValue _camerapawnreference))) false false)))

(event `InputAction|RotateBuildingLeft`
  (params (Key :type "Key Structure" :default "AnyKey"))
  (bind _ghost_building_ref (`self.Ghost Building Ref`))
  (bind (_returnvalue_roll _returnvalue_pitch _returnvalue_yaw) (`KismetMathLibrary.BreakRotator` (`self.K2_GetActorRotation` _ghost_building_ref)))
  ;[1 1 1] Place Building
  (:`Pressed`
    (if (and (`KismetSystemLibrary.IsValid` _ghost_building_ref) (`self.BuildModeActive`)) :!label _label_2
      (set `self.TurningLeft` true)
      (`self.K2_SetActorRotation` _ghost_building_ref (`KismetMathLibrary.MakeRotator` _returnvalue_roll _returnvalue_pitch (+ _returnvalue_yaw (`self.BuildingRotationRate`))) false)
      (`KismetSystemLibrary.Delay` 0.1)
      (if (`self.TurningLeft`)
        (goto _label_2))))
  (:`Released`
    (set `self.TurningLeft` false)))

(event `Key|LeftShift`
  (params (Key :type "Key Structure" :default "AnyKey"))
  ;[1 1 1] Camera Movement
  ;;[1 1 1] Move multi
  (:`Pressed`
    (set `self.FastMoveMultiplier` 2.0))
  (:`Released`
    (set `self.FastMoveMultiplier` 1.0)))

(event `InputAxisKey|MouseX`
  (params (AxisValue :type "Float (single-precision)"))
  ;[1 1 1] Camera Movement
  ;;[1 1 1] Pan X
  (`/Engine/EditorBlueprintResources/StandardMacros.Gate` true :!label _label_3
    (:`Exit`
      (`self.K2_SetActorRotation` (`self.CameraPawnReference`) (`KismetMathLibrary.MakeRotator` (.roll (`self.K2_GetActorRotation` (`self.CameraPawnReference`))) (.pitch (`self.K2_GetActorRotation` (`self.CameraPawnReference`))) (+ (.yaw (`self.K2_GetActorRotation` (`self.CameraPawnReference`))) (* (`self.PanSencitivity`) AxisValue))) false))))

(event `InputAxisKey|MouseY`
  (params (AxisValue :type "Float (single-precision)"))
  ;[1 1 1] Camera Movement
  ;;[1 1 1] Pan Y
  (`/Engine/EditorBlueprintResources/StandardMacros.Gate` true :!label _label_4
    (:`Exit`
      (`self.K2_SetActorRotation` (`self.CameraPawnReference`) (`KismetMathLibrary.MakeRotator` (.roll (`self.K2_GetActorRotation` (`self.CameraPawnReference`))) (`KismetMathLibrary.FClamp` (+ (.pitch (`self.K2_GetActorRotation` (`self.CameraPawnReference`))) (* (`self.PanSencitivity`) AxisValue)) -40.0 40.0) (.yaw (`self.K2_GetActorRotation` (`self.CameraPawnReference`)))) false))))

(event `InputAction|Pan`
  (params (Key :type "Key Structure" :default "AnyKey"))
  ;[1 1 1] Camera Movement
  ;;[1 1 1] Pan X
  (:`Pressed`
    (set `self.DisableCamNav` true)
    (goto _label_3 :!via `Open`))
  (:`Released`
    (set `self.DisableCamNav` false)
    (goto _label_3 :!via `Close`)))

(event `InputAction|Pan`
  (params (Key :type "Key Structure" :default "AnyKey"))
  ;[1 1 1] Camera Movement
  ;;[1 1 1] Pan Y
  (:`Pressed`
    (set `self.DisableCamNav` true)
    (goto _label_4 :!via `Open`))
  (:`Released`
    (set `self.DisableCamNav` false)
    (goto _label_4 :!via `Close`)))

(event `InputAction|PanPeset`
  (params (Key :type "Key Structure" :default "AnyKey"))
  (bind _camerapawnreference (`self.CameraPawnReference`))
  ;[1 1 1] Camera Movement
  ;;[1 1 1] Pan reset
  (:`Pressed`
    (`self.K2_SetActorRotation` _camerapawnreference (`KismetMathLibrary.MakeRotator` (.roll (`self.K2_GetActorRotation` _camerapawnreference)) 0.0 (.yaw (`self.K2_GetActorRotation` _camerapawnreference))) false)))

(event `InputAxisKey|MouseX`
  (params (AxisValue :type "Float (single-precision)"))
  ;[1 1 1] Camera Movement
  ;;[1 1 1] Mouse Movement
  (if (not (`self.DisableCamNav`))
    (bind (_deltax _delstay) (`self.ScreenEdgeMove` :!label _label_5))
    (`self.K2_AddActorLocalOffset` (`self.CameraPawnReference`) (`KismetMathLibrary.MakeVector` _deltax _delstay) true false)))

(event `InputAction|ZoomIn`
  (params (Key :type "Key Structure" :default "AnyKey"))
  (bind _springarm (`/Game/rts/Blueprints/CameraPawn.SpringArm` (`self.CameraPawnReference`)))
  ;[1 1 1] Camera Movement
  ;;[1 1 1] Zomm in/out
  (:`Pressed`
    (set `SpringArmComponent.TargetArmLength` (`KismetMathLibrary.FClamp` (- (`SpringArmComponent.TargetArmLength` _springarm) (`self.ZoomSenc`)) 500.0 (`self.MaxArmDist`)) _springarm)))

(event `InputAxisKey|MouseY`
  (params (AxisValue :type "Float (single-precision)"))
  ;[1 1 1] Camera Movement
  ;;[1 1 1] Mouse Movement
  (if (not (`self.DisableCamNav`))
    (goto _label_5 :!via `MouseY`)))

(event `InputAction|ZoomOut`
  (params (Key :type "Key Structure" :default "AnyKey"))
  (bind _springarm (`/Game/rts/Blueprints/CameraPawn.SpringArm` (`self.CameraPawnReference`)))
  ;[1 1 1] Camera Movement
  ;;[1 1 1] Zomm in/out
  (:`Pressed`
    (set `SpringArmComponent.TargetArmLength` (`KismetMathLibrary.FClamp` (+ (`self.ZoomSenc`) (`SpringArmComponent.TargetArmLength` _springarm)) 500.0 (`self.MaxArmDist`)) _springarm)))

(event `InputAction|ZoomReset`
  (params (Key :type "Key Structure" :default "AnyKey"))
  ;[1 1 1] Camera Movement
  ;;[1 1 1] Reset zoom
  (:`Pressed`
    (set `SpringArmComponent.TargetArmLength` 1500.0 (`/Game/rts/Blueprints/CameraPawn.SpringArm` (`self.CameraPawnReference`)))))

(fn `MovementSpeedCalculation`
  (returns (MoveSenc :type "Float (double-precision)"))
  (return (`KismetMathLibrary.FClamp` (/ (`SpringArmComponent.TargetArmLength` (`/Game/rts/Blueprints/CameraPawn.SpringArm` (`self.CameraPawnReference`))) 100.0) 5.0 20.0)))

(fn `SetCalendar`
  (params (Date :type "Array of Integer (by ref)"))
  (returns (Success :type Boolean))
  (return false))

(fn `SetClock`
  (params (Time :type "Array of Integer (by ref)"))
  (returns (Success :type Boolean))
  (return false))

(fn `SetSiteDistance`
  (returns (SiteDistance :type "Float (double-precision)"))
  (return (- (`self.SiteDistance`) (`SpringArmComponent.TargetArmLength` (`/Game/rts/Blueprints/CameraPawn.SpringArm` (`self.CameraPawnReference`))))))

(fn `UserConstructionScript`)