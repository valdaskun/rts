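; Randomized NPC character for an RTS that opens its own HUD when requested through the camera pawn controller.
; Construction script rolls sex and an enum-based name into a profile and tints the body material, though the tint re-rolls sex independently.
; The HUD request switches to UI-only input, glides the camera over by timeline, then disables navigation and opens a Tick gate to follow the NPC.
; SetIsBusy writes to the AI blackboard.
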(event `self.ReceiveBeginPlay`
  (bind _returnvalue (`AIBlueprintHelperLibrary.GetAIController` self))
  (set `self.AIControllerRef` (cast `/Game/rts/Blueprints/AI/NPC_AIController` _returnvalue :!pure true))
  (bind _ascamera_pawn_controller (cast `/Game/rts/Blueprints/CameraPawnCOntroller` (`GameplayStatics.GetPlayerController` 0)))
  (bind _output_get (set `self.ControllerRef` _ascamera_pawn_controller))
  (add `/Game/rts/Blueprints/CameraPawnCOntroller.HUDRequest` _output_get (`|CreateDelegate` :!event `Display HUD`))
  (bind _returnvalue_2 (`|CreateWidget` "/Game/rts/HUDs/NPC_HUD.NPC_HUD_C" null self))
  (set `self.NPC_HUD` _returnvalue_2))

(event `Display HUD`
  (params (Actor :type "Actor Object Reference"))
  (bind _controllerref (`self.ControllerRef`))
  (bind _npc_hud (`self.NPC_HUD`))
  (bind _camerapawnreference (`/Game/rts/Blueprints/CameraPawnCOntroller.CameraPawnReference` (`self.ControllerRef`)))
  (if (and (== Actor self) (not (`self.bHidden`)))
    (`UserWidget.AddToViewport` _npc_hud 0)
    (`WidgetBlueprintLibrary.SetInputMode_UIOnlyEx` _controllerref _npc_hud "LockOnCapture")
    (`Widget.SetIsEnabled` (`/Game/rts/Blueprints/CameraPawnCOntroller.MainHudRef` _controllerref) false)
    (bind (_direction _speed) (`Timeline|LerpLocationTimeline` :!via `PlayFromStart`)
      (:`Update`
        (`self.K2_SetActorLocation` _camerapawnreference (`/Game/rts/Libraries/FunctionLibrary.HUDLerpLocation` (`self.K2_GetActorLocation` _camerapawnreference) (`self.K2_GetActorLocation`) _speed) false false))
      (:`Finished`
        (set `/Game/rts/Blueprints/CameraPawnCOntroller.DisableCamNav` true (`self.ControllerRef`))
        (`self.OpenFollowGate`)))))

(event `self.ReceiveTick`
  (params (DeltaSeconds :type "Float (single-precision)"))
  (bind (_returnvalue_x _returnvalue_y) (`KismetMathLibrary.BreakVector` (`self.K2_GetActorLocation`)))
  (bind _camerapawnreference (`/Game/rts/Blueprints/CameraPawnCOntroller.CameraPawnReference` (`self.ControllerRef`)))
  (bind (_returnvalue_x_2 _returnvalue_y_2 _returnvalue_z) (`KismetMathLibrary.BreakVector` (`self.K2_GetActorLocation` _camerapawnreference)))
  (`/Engine/EditorBlueprintResources/StandardMacros.Gate` true :!label _label
    (:`Exit`
      (`self.K2_SetActorLocation` _camerapawnreference (`KismetMathLibrary.MakeVector` _returnvalue_x _returnvalue_y _returnvalue_z) false false))))

(event `OpenFollowGate`
  (goto _label :!via `Open`))

(event `CloseFollowGate`
  (goto _label :!via `Close`))

(fn `GetRandomName`
  (params (Sex :type "/Game/rts/Enums/NPCSex_ENUM Enum"))
  (returns (Name :type String))
  (if (`|EnumEquality` Sex "NewEnumerator0")
    (return (`|GetEnumeratorNameAsString` (enumliteral `/Game/rts/Enums/NPCNameMale_ENUM` (cast `/Game/rts/Enums/NPCNameMale_ENUM` (`KismetMathLibrary.Conv_IntToByte` (`KismetMathLibrary.RandomIntegerInRange` 0 (- (enumcount `/Game/rts/Enums/NPCNameMale_ENUM`) 1)))))))
    (else
      (return (`|GetEnumeratorNameAsString` (enumliteral `/Game/rts/Enums/NPCNameFemale_ENUM` (cast `/Game/rts/Enums/NPCNameFemale_ENUM` (`KismetMathLibrary.Conv_IntToByte` (`KismetMathLibrary.RandomIntegerInRange` 0 (- (enumcount `/Game/rts/Enums/NPCNameFemale_ENUM`) 1))))))))))

(fn `RandormNPCFeatures`
  (locals (MaterialInstance :type "MaterialInstanceDynamic Object Reference") (RandomSex :type "/Game/rts/Enums/NPCSex_ENUM Enum") (FemaleColor :type "LinearColor Structure" :default (struct :`R` 1.0 :`G` 0.1 :`B` 1.0)) (MaleColor :type "LinearColor Structure" :default (struct :`R` 0.1 :`G` 0.1 :`B` 1.0)))
  (bind _randomsex (`local.RandomSex`))
  (bind _materialinstance (`local.MaterialInstance`))
  (bind _returnvalue (enumliteral `/Game/rts/Enums/NPCSex_ENUM` (cast `/Game/rts/Enums/NPCSex_ENUM` (`KismetMathLibrary.Conv_IntToByte` (`KismetMathLibrary.RandomIntegerInRange` 0 1)))))
  (bind _returnvalue_2 (`PrimitiveComponent.CreateDynamicMaterialInstance` (`self.Mesh`) 0 "/Game/rts/Character/Materials/M_UE4Man_Body_Inst.M_UE4Man_Body_Inst"))
  (set `local.MaterialInstance` _returnvalue_2)
  (set `local.RandomSex` _returnvalue)
  (if (`|EnumEquality` _returnvalue "NewEnumerator0")
    (`MaterialInstanceDynamic.SetVectorParameterValue` _materialinstance "BodyColor" (`local.MaleColor`))
    (else
      (`MaterialInstanceDynamic.SetVectorParameterValue` _materialinstance "BodyColor" (`local.FemaleColor`))))
  (bind _name (`self.GetRandomName` _randomsex))
  (set `self.MyProfile` (make `/Game/rts/Strucs/NPCProfile_struct` _name _randomsex)))

(fn `SetIsBusy`
  (params (IsBusy :type Boolean))
  (`BlackboardComponent.SetValueAsBool` (`AIBlueprintHelperLibrary.GetBlackboard` (`self.AIControllerRef`)) (`self.IsBusy`) IsBusy)
  (return))

(fn `UserConstructionScript`
  (`self.RandormNPCFeatures`))