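; Base building actor for the RTS that shows a building HUD when the player controller requests it for this building.
; The construction script applies the display mesh and fits the entrance and collision box to it.
; On BeginPlay it binds to the CameraPawnController's HUD request event and pre-creates a Building_HUD widget, adding it to the viewport only when the requested actor is itself.
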(event `self.ReceiveBeginPlay`
  (bind _ascamera_pawn_controller (cast `/Game/rts/Blueprints/CameraPawnCOntroller` (`GameplayStatics.GetPlayerController` 0)))
  (bind _output_get (set `self.ControllerRef` _ascamera_pawn_controller))
  (add `/Game/rts/Blueprints/CameraPawnCOntroller.HUDRequest` _output_get (`|CreateDelegate` :!event `Display HUD`))
  (bind _returnvalue (`|CreateWidget` "/Game/rts/HUDs/Building_HUD.Building_HUD_C"))
  (set `self.BuildinHUD` _returnvalue))

(event `Display HUD`
  (params (Actor :type "Actor Object Reference"))
  (if (== Actor self)
    (`UserWidget.AddToViewport` (`self.BuildinHUD`) 0)))

(fn `UserConstructionScript`
  (`StaticMeshComponent.SetStaticMesh` (`self.StaticMesh`) (`self.DisplayMesh`))
  (`/Game/rts/Libraries/FunctionLibrary.SetBuildingEntrance` (`self.Entrance`) (`self.StaticMesh`))
  (`/Game/rts/Libraries/FunctionLibrary.SetBuildingCollisionBox` (`self.Collision`) (`self.StaticMesh`)))