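; Spawn_BP is an NPC that randomizes its sex, name and body color in the construction script.
; It creates a dynamic material on the mesh, tints BodyColor by sex, and stores name and sex in MyProfile.
; The color branch re-rolls the random sex, so color can disagree with the profile.
; Both GetRandomName branches draw from the female name enum, leaving the male lookup unused.
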(fn `GetRandomName`
  (params (Sex :type "/Game/rts/Enums/NPCSex_ENUM Enum"))
  (returns (Name :type String))
  (bind _returnvalue (`|GetEnumeratorNameAsString` (enumliteral `/Game/rts/Enums/NPCNameFemale_ENUM` (cast `/Game/rts/Enums/NPCNameFemale_ENUM` (`KismetMathLibrary.Conv_IntToByte` (`KismetMathLibrary.RandomIntegerInRange` 0 (- (enumcount `/Game/rts/Enums/NPCNameFemale_ENUM`) 1)))))))
  (if (`|EnumEquality` Sex "NewEnumerator0")
    (return _returnvalue)
    (else
      (return _returnvalue))))

(fn `RandormNPCFeatures`
  (locals (MaterialInstance :type "MaterialInstanceDynamic Object Reference") (RandomSex :type "/Game/rts/Enums/NPCSex_ENUM Enum") (FemaleColor :type "LinearColor Structure" :default (struct :`R` 1.0 :`G` 0.1 :`B` 1.0)) (MaleColor :type "LinearColor Structure" :default (struct :`R` 0.1 :`G` 0.1 :`B` 1.0)))
  (bind _randomsex (`local.RandomSex`))
  (bind _materialinstance (`local.MaterialInstance`))
  (bind _returnvalue (enumliteral `/Game/rts/Enums/NPCSex_ENUM` (cast `/Game/rts/Enums/NPCSex_ENUM` (`KismetMathLibrary.Conv_IntToByte` (`KismetMathLibrary.RandomIntegerInRange` 0 1)))))
  (bind _returnvalue_2 (`PrimitiveComponent.CreateDynamicMaterialInstance` (`self.Mesh`) 0 "/Game/rts/Character/Materials/M_UE4Man_Body_Inst.M_UE4Man_Body_Inst"))
  (set `local.MaterialInstance` _returnvalue_2)
  (set `local.RandomSex` _returnvalue)
  (if (`|EnumEquality` _returnvalue "NewEnumerator0")
    (`MaterialInstanceDynamic.SetVectorParameterValue` _materialinstance "BodyColor" (`local.MaleColor`))
    (else
      (`MaterialInstanceDynamic.SetVectorParameterValue` _materialinstance "BodyColor" (`local.FemaleColor`))))
  (bind _name (`self.GetRandomName` _randomsex))
  (set `self.MyProfile` (make `/Game/rts/Strucs/NPCProfile_struct` _name _randomsex)))

(fn `UserConstructionScript`
  (`self.RandormNPCFeatures`))